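; Game manager that tracks wave progress and the igloo's life as the player's health.
; IglooTakeDamage subtracts from current life, then Defeat adds the UW_Defeat widget to the viewport once life reaches zero or below.
; Tick polls the Enemies list, setting CanSpawnNextWave when it empties after having held enemies.
; RemoveEnemyFromList removes enemies from that list, while BeginPlay initializes the wave counter and life.
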(event EventTick
  (params (DeltaSeconds :type Float%20%28single-precision%29))
  (CallFunction|EndOfWave))

(event EventBeginPlay
  (Variables|Default|SetCurrentWave 0)
  (Variables|Default|SetPlayerCurrentLife (Variables|Default|GetPlayerMaxLife)))

(fn ConstructionScript)

(fn Defeat
  (if (<= (Variables|Default|GetPlayerCurrentLife) 0)
    (bind _returnvalue (UserInterface|CreateWidget "/Game/UI/UW_Defeat.UW_Defeat_C"))
    (UserInterface|Viewport|AddtoViewport _returnvalue 0)))

(fn IglooTakeDamage
  (params (Damage :type Integer))
  (Variables|Default|SetPlayerCurrentLife (- (Variables|Default|GetPlayerCurrentLife) Damage))
  (CallFunction|Defeat))

(fn EndOfWave
  (if (Utilities|Array|IsNotEmpty (Variables|Default|GetEnemies))
    (Variables|Default|SetEnemiesHasSpawn true)
    (elif (and (Variables|Default|GetEnemiesHasSpawn) (Utilities|Array|IsEmpty (Variables|Default|GetEnemies)))
      (Variables|Default|SetCanSpawnNextWave true))))

(fn RemoveEnemyfromList
  (params (Enemy :type C%20Enemy%20Object%20Reference))
  (Utilities|Array|RemoveItem (Variables|Default|GetEnemies) Enemy))