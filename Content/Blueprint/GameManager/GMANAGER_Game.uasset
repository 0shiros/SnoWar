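; Game manager Blueprint that tracks igloo player life and the wave's enemy list.
; IglooTakeDamage subtracts damage from player life and prints a defeat message once it reaches zero or below.
; Every tick, EndOfWave flags that enemies have spawned, then prints an end-of-wave message while the list is empty again.
; Enemies leave the list through RemoveEnemyFromList; both outcomes are only debug prints.
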(event EventTick
  (params (DeltaSeconds :type Float%20%28single-precision%29))
  (CallFunction|EndOfWave))

(fn ConstructionScript)

(fn Defeat
  (if (<= (Variables|Default|GetPlayerLife) 0)
    (Development|PrintString "Defeat")))

(fn IglooTakeDamage
  (params (Damage :type Integer))
  (Variables|Default|SetPlayerLife (- (Variables|Default|GetPlayerLife) Damage))
  (CallFunction|Defeat))

(fn EndOfWave
  (if (Utilities|Array|IsNotEmpty (Variables|Default|GetEnemies))
    (Variables|Default|SetEnemiesHasSpawn true)
    (elif (and (Variables|Default|GetEnemiesHasSpawn) (Utilities|Array|IsEmpty (Variables|Default|GetEnemies)))
      (Development|PrintString "EndOfWave"))))

(fn RemoveEnemyfromList
  (params (Enemy :type C%20Enemy%20Object%20Reference))
  (Utilities|Array|RemoveItem (Variables|Default|GetEnemies) Enemy))