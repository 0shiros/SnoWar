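; PC_Snouw is the player controller that handles movement input for the C_Snouw character.
; On start it caches player 0's character as C_Snouw and, if that cast succeeds, adds the IMC_Snouw Enhanced Input mapping context.
; The forward/backward and right/left input actions feed their values into the character's movement input along its own forward and right vectors.
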(event Custom|Start
  (bind _asc_snouw (Utilities|Casting|CastToC_Snouw (Game|GetPlayerCharacter 0)))
  (Variables|Default|SetAs%20C%20Snouw _asc_snouw)
  (Input|AddMappingContext (PlayerController|LocalPlayerSubsystems|GetEnhancedInputLocalPlayerSubsystem self) "/Game/Input/IMC_Snouw.IMC_Snouw" 0 "(bIgnoreAllPressedKeysUntilRelease=True,bForceImmediately=False,bNotifyUserSettings=False)"))

(event Input|EnhancedActionEvents|EnhancedInputActionIAC_RightLeft
  (params (ActionValue :type Float%20%28double-precision%29) (ElapsedSeconds :type Float%20%28double-precision%29) (TriggeredSeconds :type Float%20%28double-precision%29) (InputAction :type Input%20Action%20Object%20Reference :default "/Game/Input/IAC_RightLeft.IAC_RightLeft"))
  (bind _as_c_snouw (Variables|Default|GetAs%20C%20Snouw))
  (Pawn|Input|AddMovementInput _as_c_snouw (Transformation|GetActorRightVector _as_c_snouw) ActionValue false))

(event Input|EnhancedActionEvents|EnhancedInputActionIAC_ForwardBackward
  (params (ActionValue :type Float%20%28double-precision%29) (ElapsedSeconds :type Float%20%28double-precision%29) (TriggeredSeconds :type Float%20%28double-precision%29) (InputAction :type Input%20Action%20Object%20Reference :default "/Game/Input/IAC_ForwardBackward.IAC_ForwardBackward"))
  (bind _as_c_snouw (Variables|Default|GetAs%20C%20Snouw))
  (Pawn|Input|AddMovementInput _as_c_snouw (Transformation|GetActorForwardVector _as_c_snouw) ActionValue false))

(fn ConstructionScript)